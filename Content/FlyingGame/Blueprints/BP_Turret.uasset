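; BP_Turret is a turret in FlyingGame that aims its top mesh at the nearest visible pawn; it has no firing logic.
; Each Tick, FindBestTarget sphere-overlaps pawns within SensingRange, keeps the closest with line of sight, and debug-prints its name.
; UpdateTurretRotation then feeds RInterpToConstant with Current and Target swapped, so the top snaps to within one RotateSpeed step of the target instead of turning gradually.
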(event `self.ReceiveTick`
  (params (DeltaSeconds :type "Float (single-precision)"))
  (`self.FindBestTarget`)
  (`KismetSystemLibrary.PrintString` (`KismetSystemLibrary.GetDisplayName` (`self.Target`)))
  (`self.Target`
    (:`then`
      (`self.Update Turret Rotation` DeltaSeconds))
    (:`else`)))

(fn `FindBestTarget`
  (locals (`bestDistance (local)` :type "Float (double-precision)") (`currentDistance (local)` :type "Float (double-precision)") (`bestTarget (local)` :type "Actor Object Reference") (`currentTarget (local)` :type "Actor Object Reference"))
  (set `local.bestDistance (local)` (+ (`self.sensingRange`) 1.0))
  (bind _outactors (`KismetSystemLibrary.SphereOverlapActors` (`self.K2_GetActorLocation`) (`self.sensingRange`) (`|MakeArray` "ObjectTypeQuery3" :!type "EObjectTypeQuery Enum") "/Script/Engine.Actor"))
  (for _array_element _outactors
    (bind _output_get (set `local.currentTarget (local)` _array_element))
    (bind _output_get_2 (set `local.currentDistance (local)` (`self.GetDistanceTo` _output_get self)))
    (if (or (< _output_get_2 (`local.bestDistance (local)`)) (not (`KismetSystemLibrary.IsValid` (`local.bestTarget (local)`))))
      (bind _result (`/Game/FlyingGame/Blueprints/MyFunctionLibrary.hasLineofSight` (`SceneComponent.K2_GetComponentLocation` (`self.StaticMeshTop`)) (`self.K2_GetActorLocation` (`local.currentTarget (local)`)) (`|MakeArray` self (`local.currentTarget (local)`) :!type "Actor Object Reference")))
      (if _result
        (set `local.bestTarget (local)` (`local.currentTarget (local)`))
        (set `local.bestDistance (local)` (`local.currentDistance (local)`)))))
  (set `self.Target` (`local.bestTarget (local)`)))

(fn `Update Turret Rotation`
  (params (`Delta Seconds` :type "Float (double-precision)"))
  (`SceneComponent.K2_SetWorldRotation` (`self.StaticMeshTop`) (`KismetMathLibrary.RInterpTo_Constant` (`KismetMathLibrary.FindLookAtRotation` (`SceneComponent.K2_GetComponentLocation` (`self.StaticMeshTop`)) (`self.K2_GetActorLocation` (`self.Target`))) (`SceneComponent.K2_GetComponentRotation` (`self.StaticMeshTop`)) (`local.Delta Seconds`) (`self.Rotate Speed`)) false false))

(fn `UserConstructionScript`)